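; AI controller Blueprint for the angel enemy, named for Behavior Tree use, that tracks perception of the player.
; Perception updates store the perceived actor and, when an actor tagged Player is no longer sensed, start an 8-second one-shot timer bound to LoseSight.
; It is unfinished: LoseSight and both key-update functions are empty, successful sensing has no further handling, and no tree is run here.
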(event `self.PerceptionComp.OnTargetPerceptionUpdated`
  (params (Actor :type "Actor Object Reference") (Stimulus :type "AIStimulus Structure"))
  (set `self.PerceivedActor` Actor)
  (if (`self.ActorHasTag` Actor "Player")
    (if (not (`.bSuccessfullySensed` (break `AIStimulus` Stimulus)))
      (bind _returnvalue (`KismetSystemLibrary.K2_SetTimerDelegate` (delegate `LoseSight`) 8.0))
      (set `self.LoseSIghtTimer` _returnvalue))))

(event `LoseSight`)

(fn `UpdateSightKey`
  (params (HasLineOfSight :type Boolean)))

(fn `UpdateTargetKey`)

(fn `UserConstructionScript`
  (`parent.UserConstructionScript`))